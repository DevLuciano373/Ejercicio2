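; BP_Arquero is an archer actor that can face a target and shoot arrows, through functions with no caller inside this Blueprint.
; ApuntarPersonaje rotates the whole actor toward a given location using a look-at rotation, with debug prints.
; SetVelocidadFlecha scales the Velocidad vector by a factor into VelocidadDeFlecha.
; SpawnFlecha spawns BP_Flecha at the actor's location and passes that velocity to it.
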(fn `ApuntarPersonaje`
  (params (DireccionPersonaje :type "Vector Structure"))
  (bind _returnvalue (`KismetMathLibrary.FindLookAtRotation` (`self.K2_GetActorLocation`) DireccionPersonaje))
  (`KismetSystemLibrary.PrintString` "rotando personaje")
  (`KismetSystemLibrary.PrintString` (`KismetStringLibrary.Conv_RotatorToString` _returnvalue))
  (`self.K2_SetActorRotation` _returnvalue))

(fn `Set Velocidad Flecha`
  (params (Velocidad :type "Vector Structure") (FactorVelocidad :type "Float (double-precision)"))
  (bind _output_get (set `self.FactorVelocidad` FactorVelocidad))
  (set `self.VelocidadDeFlecha` (`KismetMathLibrary.MakeVector` (* Velocidad_X _output_get) (* Velocidad_Y _output_get) (* Velocidad_Z _output_get))))

(fn `SpawnFlecha`
  (`|SpawnActorFromClass` "/Game/BP_Flecha.BP_Flecha_C" (`KismetMathLibrary.MakeTransform` (`self.K2_GetActorLocation`)) "Undefined" "MultiplyWithRoot" null (`self.VelocidadDeFlecha`) null))

(fn `UserConstructionScript`)